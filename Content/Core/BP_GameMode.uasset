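; BP_GameMode is the game mode Blueprint that starts the game UI once the player controller reports that it is initialised.
; On BeginPlay it casts player controller 0 to BP_PlayerController, caches the reference, then binds an event to that controller's initialised notification.
; Its OnPlayerControllerInitialised handler calls InitialiseUIGame on the cached controller.
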(event `self.ReceiveBeginPlay`
  ;[1 1 1] Initialise
  (`self.SetReferences`)
  (`self.BindToEvents`))

(fn `BindToEvents`
  ;[1 1 1] Bind to Events
  (add `/Game/Core/BP_PlayerController.PlayerControllerInitialised` (`self.PlayerController`) (`|CreateDelegate` :!event `OnPlayerControllerInitialised`)))

(fn `OnPlayerControllerInitialised`
  ;[1 1 1] Event Handler
  (`/Game/Core/BP_PlayerController.InitialiseUIGame` (`self.PlayerController`)))

(fn `SetReferences`
  ;[1 1 1] Set References
  (bind _asbp_player_controller (cast `/Game/Core/BP_PlayerController` (`GameplayStatics.GetPlayerController` 0)))
  (set `self.PlayerController` _asbp_player_controller))

(fn `UserConstructionScript`)