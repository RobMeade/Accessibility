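; Turret NPC that tracks and shoots at the player, with a health bar widget that turns to face them.
; On BeginPlay it takes health from player preferences and ranges from the GameInstance.
; Tick smoothly aims via overlap polling (both overlap events clear TargetInRange) and runs a looping timer spawning projectiles while the player is within firing distance.
; Damage lowers clamped health and updates the bar, with no death handling.
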(event `self.ReceiveBeginPlay`
  ;[1 1 1] Initialise
  (`self.SetReferences`)
  (`self.CreateHealthBarWidget`)
  (`self.ApplyPlayerPreferences`)
  (`self.SetRanges`))

(event `self.ReceiveTick`
  (params (DeltaSeconds :type "Float (single-precision)"))
  ;[1 1 1] Tick
  (`self.RotateHealthBarToPlayer`)
  (`self.DetermineAimingAction`)
  (`self.DetermineFiringAction`))

(event `self.TargettingRange.OnComponentBeginOverlap`
  (params (OverlappedComponent :type "PrimitiveComponent Object Reference") (OtherActor :type "Actor Object Reference") (OtherComp :type "PrimitiveComponent Object Reference") (OtherBodyIndex :type Integer) (bFromSweep :type Boolean) (SweepResult :type "HitResult Structure (by ref)"))
  ;[1 1 1] Targetting Range
  (if (== OtherActor (`self.Target`))
    (set `self.TargetInRange` false)))

(event `self.TargettingRange.OnComponentEndOverlap`
  (params (OverlappedComponent :type "PrimitiveComponent Object Reference") (OtherActor :type "Actor Object Reference") (OtherComp :type "PrimitiveComponent Object Reference") (OtherBodyIndex :type Integer))
  ;[1 1 1] Targetting Range
  (if (== OtherActor (`self.Target`))
    (set `self.TargetInRange` false)))

(event `/Game/Core/Characters/Player/IDamageable.TakeDamage`
  (params (Damage :type Integer))
  (`self.DecreaseHealth` Damage))

(fn `AimAtTarget`
  (bind (_returnvalue_roll _returnvalue_pitch _returnvalue_yaw) (`KismetMathLibrary.BreakRotator` (`KismetMathLibrary.FindLookAtRotation` (`SceneComponent.K2_GetComponentLocation` (`self.Turret`)) (`SceneComponent.K2_GetComponentLocation` (`Character.CapsuleComponent` (`self.Target`))))))
  ;[1 1 1] Aim At Target
  (`SceneComponent.K2_SetWorldRotation` (`self.Turret`) (`KismetMathLibrary.RInterpTo` (`SceneComponent.K2_GetComponentRotation` (`self.Turret`)) (`KismetMathLibrary.MakeRotator` 0.0 _returnvalue_pitch _returnvalue_yaw) (`GameplayStatics.GetWorldDeltaSeconds`) 5.0) false false))

(fn `ApplyPlayerPreferences`
  (bind (_cognitivepreferences_playerhealthpoints _cognitivepreferences_healthregenerates _cognitivepreferences_invincibility _cognitivepreferences_enemyhealthpoints) (break `/Game/Core/Structures/SPlayerPreferencesCognitive` (`/Game/Core/BP_GameInstance.GetPlayerPreferencesCognitive` (`self.GameInstance`))))
  ;[1 1 1] Apply Player Preferences
  (`self.SetHealth` _cognitivepreferences_enemyhealthpoints))

(fn `CreateHealthBarWidget`
  ;[1 1 1] Create Health Bar Widget
  (bind _returnvalue (`|CreateWidget` "/Game/Core/Characters/NPC/WBP_NPCHealthBar.WBP_NPCHealthBar_C"))
  (bind _output_get (set `self.HealthBarWidget` _returnvalue))
  (`WidgetComponent.SetWidget` (`self.HealthBar`) _output_get))

(fn `DecreaseHealth`
  (params (Value :type Integer))
  ;[1 1 1] Decrease Health
  (bind _output_get (set `self.Health` (`KismetMathLibrary.Clamp` (- (`self.Health`) Value) 0 (`self.MaximumHealth`))))
  (`self.UpdateHealthBar` _output_get))

(fn `DetermineAimingAction`
  ;[1 1 1] Determine Aiming Action
  (`self.IsTargetAlreadyWithingTargettingRange`)
  (if (`self.TargetInRange`)
    (`self.AimAtTarget`)))

(fn `DetermineFiringAction`
  ;[1 1 1] Determine Firing Action
  (if (`self.IsTargetWithinFiringRange`)
    (`self.StartFiringAtTarget`)
    (else
      (`self.StopFiringAtTarget`))))

(fn `Fire`
  (bind (_returnvalue_location _returnvalue_rotation) (`KismetMathLibrary.BreakTransform` (`SceneComponent.K2_GetComponentToWorld` (`self.FiringPoint`))))
  ;[1 1 1] Fire
  (`|SpawnActorFromClass` "/Game/Core/Characters/NPC/BP_NPCProjectile.BP_NPCProjectile_C" (`KismetMathLibrary.MakeTransform` _returnvalue_location _returnvalue_rotation) "AlwaysSpawn" "OverrideRootScale" null null))

(fn `IsTargetAlreadyWithingTargettingRange`
  ;[1 1 1] Is Target Already With Targetting Range (covers BeginOverlap Event not triggering if player is spawned within TargettingRange volume)
  (if (`self.TargetInRange`)
    _
    (elif (`self.IsOverlappingActor` (`self.Target`))
      (set `self.TargetInRange` true))))

(fn `IsTargetWithinFiringRange`
  (returns (InRange :type Boolean))
  ;[1 1 1] Is Target within Firing Range?
  (return (<= (`self.GetDistanceTo` (`self.Target`)) (`self.FiringRange`))))

(fn `RotateHealthBarToPlayer`
  (bind (_returnvalue_roll _returnvalue_pitch _returnvalue_yaw) (`KismetMathLibrary.BreakRotator` (`KismetMathLibrary.FindLookAtRotation` (`SceneComponent.K2_GetComponentLocation` (`self.HealthBar`)) (`SceneComponent.K2_GetComponentLocation` (`Actor.RootComponent` (`self.Target`))))))
  ;[1 1 1] Rotate Health Bar to Player
  (`SceneComponent.K2_SetWorldRotation` (`self.HealthBar`) (`KismetMathLibrary.MakeRotator` _returnvalue_roll 0.0 _returnvalue_yaw) false false))

(fn `SetHealth`
  (params (Health :type "Float (double-precision)"))
  ;[1 1 1] Set Health
  (bind _output_get (set `self.MaximumHealth` (`KismetMathLibrary.FTrunc` (* Health 100.0))))
  (bind _output_get_2 (set `self.Health` _output_get))
  (`self.UpdateHealthBar` _output_get_2))

(fn `SetRanges`
  ;[1 1 1] Set Ranges
  (`SphereComponent.SetSphereRadius` (`self.TargettingRange`) (`/Game/Core/BP_GameInstance.NPCTargettingRange` (`self.GameInstance`)) true)
  (set `self.FiringRange` (`/Game/Core/BP_GameInstance.NPCFiringRange` (`self.GameInstance`))))

(fn `SetReferences`
  ;[1 1 1] Set References
  (bind _asbp_game_instance (cast `/Game/Core/BP_GameInstance` (`GameplayStatics.GetGameInstance`)))
  (set `self.GameInstance` _asbp_game_instance)
  (bind _asbp_player_character (cast `/Game/Core/Characters/Player/BP_PlayerCharacter` (`GameplayStatics.GetPlayerCharacter` 0)))
  (set `self.Target` _asbp_player_character))

(fn `StartFiringAtTarget`
  ;[1 1 1] Start Firing at Target
  (if (not (`KismetSystemLibrary.K2_TimerExistsHandle` (`self.FireTimerHandler`)))
    (bind _returnvalue (`KismetSystemLibrary.K2_SetTimer` null "Fire" 3.0 true))
    (set `self.FireTimerHandler` _returnvalue)))

(fn `StopFiringAtTarget`
  ;[1 1 1] Stop Firing at Target
  (`KismetSystemLibrary.K2_ClearAndInvalidateTimerHandle` (`self.FireTimerHandler`)))

(fn `UpdateHealthBar`
  (params (Health :type Integer))
  (bind (_cognitivepreferences_playerhealthpoints _cognitivepreferences_healthregenerates _cognitivepreferences_invincibility _cognitivepreferences_enemyhealthpoints) (break `/Game/Core/Structures/SPlayerPreferencesCognitive` (`/Game/Core/BP_GameInstance.GetPlayerPreferencesCognitive` (`self.GameInstance`))))
  ;[1 1 1] Update Health Bar
  (`/Game/Core/Characters/NPC/WBP_NPCHealthBar.SetValue` (`self.HealthBarWidget`) (/ (/ (`KismetMathLibrary.Conv_IntToDouble` Health) 100.0) _cognitivepreferences_enemyhealthpoints)))

(fn `UserConstructionScript`)