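; BP_GameMode_Game is the game mode for gameplay, handling music playback and startup of the in-game UI.
; On BeginPlay it caches the game instance and player controller, binds to the controller's initialised event, and starts the music.
; Music volume comes from saved player preferences, with near-zero values replaced by a minimum safe multiplier.
; Once the player controller reports it is initialised, the mode tells it to build the game UI.
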(event `self.ReceiveBeginPlay`
  ;[1 1 1] Initialise
  (`self.SetReferences`)
  (`self.BindToEvents`)
  (`self.PlayMusic`))

(fn `BindToEvents`
  ;[1 1 1] Bind to Events
  (add `/Game/Core/Characters/BP_PlayerController.PlayerControllerInitialised` (`self.PlayerController`) (`|CreateDelegate` :!event `OnPlayerControllerInitialised`)))

(fn `GetSafeVolumeMultiplier`
  (params (Volume :type "Float (double-precision)"))
  (returns (SafeVolumeMultiplier :type "Float (double-precision)"))
  ;[1 1 1] Get Safe Volume Multiplier
  (if (`KismetMathLibrary.NearlyEqual_FloatFloat` Volume)
    (return (`/Game/Core/BP_GameInstance.MinimumSafeVolumeMultiplier` (`self.GameInstance`)))
    (else
      (return (`local.Volume`)))))

(fn `OnPlayerControllerInitialised`
  ;[1 1 1] Event Handler
  (`/Game/Core/Characters/BP_PlayerController.InitialiseUIGame` (`self.PlayerController`)))

(fn `PlayMusic`
  (bind (_playerpreferences_game _playerpreferences_visual _playerpreferences_auditory) (break `/Game/Core/Structures/SPlayerPreferences` (`/Game/Core/BP_GameInstance.PlayerPreferences` (`self.GameInstance`))))
  ;[1 1 1] Play Music
  (`AudioComponent.SetVolumeMultiplier` (`self.AudioMusic`) (`self.GetSafeVolumeMultiplier` (`.MusicVolume_2_402608334FBC7DD93F67028FFF16164E` (break `/Game/Core/Structures/SPlayerPreferencesAuditory` _playerpreferences_auditory))))
  (`AudioComponent.SetSound` (`self.AudioMusic`) (`/Game/Core/BP_GameInstance.MusicGame` (`self.GameInstance`)))
  (`AudioComponent.Play` (`self.AudioMusic`) 0.0))

(fn `SetReferences`
  ;[1 1 1] Set References
  (bind _asbp_game_instance (cast `/Game/Core/BP_GameInstance` (`GameplayStatics.GetGameInstance`)))
  (set `self.GameInstance` _asbp_game_instance)
  (bind _asbp_player_controller (cast `/Game/Core/Characters/BP_PlayerController` (`GameplayStatics.GetPlayerController` 0)))
  (set `self.PlayerController` _asbp_player_controller))

(fn `UserConstructionScript`)